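; Game instance for Frenzy Grounds that handles hosting and joining multiplayer sessions, with a LAN toggle.
; HostMatch creates a session sized by the player count and, on success, opens the lobby menu level as a listen server.
; FindMatch searches for a single session and immediately joins the first result.
; TrainMatch is an empty stub, and a sessions-found call is left unconnected.
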(event Custom|TrainMatch)

(event Custom|HostMatch
  (params (NumPlayers :type Integer))
  (|Session (Game|GetPlayerController 0) NumPlayers (Variables|Default|GetUseLAN)
    (:OnSuccess
      (Game|OpenLevel(byObjectReference) "/Game/UI/LobbyMenu/LobbyMenuLevel.LobbyMenuLevel" true "?listen"))))

(event Custom|FindMatch
  (bind _results (|FindSessions (Game|GetPlayerController 0) 1 (Variables|Default|GetUseLAN))
    (:OnSuccess
      (|JoinSession (Game|GetPlayerController 0) (Utilities|Array|Get(acopy) _results)))))